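; Turret pawn that turns toward a set target and can be destroyed by beam hits.
; Each tick, while active, torso yaw and gun pitch ease toward target angles at capped speeds, with pitch clamped and guns pivoting around an offset.
; BeamActor overlaps spend remaining hits, then trigger scattered explosions, remove torso and guns, swap base material and report the indicator.
; Shoot sets a ready flag, but PerformShooting is empty.
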(event OnComponentBeginOverlap(Base)
  (params (OverlappedComponent :type Primitive%20Component%20Object%20Reference) (OtherActor :type Actor%20Object%20Reference) (OtherComp :type Primitive%20Component%20Object%20Reference) (OtherBodyIndex :type Integer) (bFromSweep :type Boolean) (SweepResult :type Hit%20Result%20Structure%20%28by%20ref%29))
  (Update|DoBeamDamage OtherActor))

(event OnComponentBeginOverlap(Torzo)
  (params (OverlappedComponent :type Primitive%20Component%20Object%20Reference) (OtherActor :type Actor%20Object%20Reference) (OtherComp :type Primitive%20Component%20Object%20Reference) (OtherBodyIndex :type Integer) (bFromSweep :type Boolean) (SweepResult :type Hit%20Result%20Structure%20%28by%20ref%29))
  (Update|DoBeamDamage OtherActor))

(event OnComponentBeginOverlap(Guns)
  (params (OverlappedComponent :type Primitive%20Component%20Object%20Reference) (OtherActor :type Actor%20Object%20Reference) (OtherComp :type Primitive%20Component%20Object%20Reference) (OtherBodyIndex :type Integer) (bFromSweep :type Boolean) (SweepResult :type Hit%20Result%20Structure%20%28by%20ref%29))
  (Update|DoBeamDamage OtherActor))

(event EventBeginPlay)

(event EventTick
  (params (DeltaSeconds :type Float%20%28single-precision%29))
  (if (Variables|Health|GetIsActive)
    (Utilities|FlowControl|Sequence
      (:then_0
        (CallFunction|UpdateRotations DeltaSeconds))
      (:then_1
        (if (Variables|Default|GetisReadyToShoot)
          (CallFunction|PerformShooting DeltaSeconds))))))

(event Collision|EventHit
  (params (MyComp :type Primitive%20Component%20Object%20Reference) (Other :type Actor%20Object%20Reference) (OtherComp :type Primitive%20Component%20Object%20Reference) (bSelfMoved :type Boolean) (HitLocation :type Vector :default "0, 0, 0") (HitNormal :type Vector :default "0, 0, 0") (NormalImpulse :type Vector :default "0, 0, 0") (Hit :type Hit%20Result%20Structure%20%28by%20ref%29))
  (Development|PrintString "turret hit"))

(fn ConstructionScript
  (bind _turretscale (Variables|Settings|GetTurretScale))
  (Transformation|SetActorScale3D (Math|Vector|MakeVector _turretscale _turretscale _turretscale)))

(fn DoBeamDamage
  (params (Object :type Object%20Object%20Reference))
  (if (Variables|Health|GetIsActive)
    (bind _asbeam_actor (Utilities|Casting|CastToBeamActor Object))
    (Effects|SpawnEmitteratLocation "/Game/StarterContent/Particles/P_Explosion.P_Explosion" (Transformation|GetActorLocation _asbeam_actor))
    (Actor|DestroyActor _asbeam_actor)
    (bind _result (Math|Integer|DecrementInt (Variables|Health|GetRemainingHits))
      (:%20%20
        (if (<= _result 0)
          (CallFunction|DestroyItself))))))

(fn DestroyItself
  (bind _extendexplosions (Variables|Settings|GetExtendExplosions))
  (for _index (range 1 20)
    (Effects|SpawnEmitteratLocation "/Game/StarterContent/Particles/P_Explosion.P_Explosion" (Math|Random|RandomPointinBoundingBox (Transformation|GetWorldLocation (Variables|Default|GetGuns)) (Math|Vector|MakeVector _extendexplosions _extendexplosions _extendexplosions)) (Math|Random|RandomRotator true)))
  (Components|DestroyComponent (Variables|Default|GetTorzo))
  (Rendering|Material|SetMaterial (Variables|Default|GetBase) 0 "/Game/Materials/GameObjects/TurretDestroyed.TurretDestroyed")
  (Variables|Health|SetIsActive false)
  (Default|CallTurretDestroyed (Variables|Default|GetInfoIndicator)))

(fn UpdateYaw
  (params (Yaw :type Float%20%28single-precision%29))
  (Transformation|SetRelativeRotation (Variables|Default|GetTorzo) (Math|Rotator|MakeRotator 0.0 0.0 Yaw) false false))

(fn UpdatePitch
  (params (A :type Float%20%28single-precision%29))
  (bind _returnvalue (Math|Rotator|MakeRotator 0.0 A 0.0))
  (bind _gunsoffset (Variables|Settings|GetGunsOffset))
  (Transformation|SetRelativeLocationAndRotation (Variables|Default|GetGuns) (+ (Math|Vector|RotateVector (* _gunsoffset -1.0) _returnvalue) _gunsoffset) _returnvalue false false))

(fn GetShootingSource
  (params (UseScaling :type Boolean))
  (bind _output_get (LocalVariables|Setoffset (Variables|Settings|GetGunsOffset)))
  (if UseScaling
    (LocalVariables|Setoffset (* _output_get (Variables|Settings|GetTurretScale))))
  (return (+ (Transformation|GetActorLocation) (Math|Vector|RotateVector (LocalVariables|Getoffset) (Transformation|GetWorldRotation (Variables|Default|GetTorzo))))))

(fn SetTargetto
  (params (Target :type Vector))
  (bind _output_get (Variables|Default|SetCurrentShootingTarget Target))
  (Variables|CurrentState|SetTargetPitch (.Pitch (Math|Rotator|BreakRotator (Math|Rotator|CombineRotators (Math|Rotator|FindLookatRotation _output_get (CallFunction|GetShootingSource true)) (Class|KismetMathLibrary|NegateRotator (Transformation|GetWorldRotation (Variables|Default|GetRoot)))))))
  (Variables|CurrentState|SetTargetYaw (.Yaw (Math|Rotator|BreakRotator (Math|Rotator|CombineRotators (Math|Rotator|FindLookatRotation _output_get (CallFunction|GetShootingSource true)) (Class|KismetMathLibrary|NegateRotator (Transformation|GetWorldRotation (Variables|Default|GetRoot))))))))

(fn GetShootingTarget
  (params (IsRight :type Boolean))
  (if IsRight
    (LocalVariables|SetMultipl "1.000000,-1.000000,1.000000")
    (else
      (LocalVariables|SetMultipl "1.000000,1.000000,1.000000")))
  (return (+ (CallFunction|GetShootingSource true) (Math|Vector|RotateVector (* (LocalVariables|GetDefaultValue) (LocalVariables|GetMultipl)) (Transformation|GetWorldRotation (Variables|Default|GetGuns))))))

(fn Shoot
  (Variables|Default|SetisReadyToShoot true))

(fn PerformShooting
  (params (Delta :type Float%20%28single-precision%29)))

(fn UpdateRotations
  (params (Delta :type Float%20%28single-precision%29))
  (bind _pitchspeedpersec (Variables|Settings|GetPitchSpeedPerSec))
  (bind _pitchclamp (Variables|Settings|GetPitchClamp))
  (bind _yawspeedpersec (Variables|Settings|GetYawSpeedPerSec))
  (bind (_x _y) (Math|Vector2D|BreakVector2D _pitchclamp))
  (Utilities|FlowControl|Sequence
    (:then_0
      (if (!= (- (Variables|CurrentState|GetTargetYaw) (Variables|CurrentState|GetYaw)) 0.0)
        (bind _output_get (Variables|CurrentState|SetYaw (+ (Variables|CurrentState|GetYaw) (* (Math|Float|Clamp(Float) (- (Variables|CurrentState|GetTargetYaw) (Variables|CurrentState|GetYaw)) (* _yawspeedpersec -1.0) _yawspeedpersec) Delta))))
        (Update|UpdateYaw _output_get)))
    (:then_1
      (if (!= (- (Variables|CurrentState|GetTargetPitch) (Variables|CurrentState|GetPitch)) 0.0)
        (bind _output_get_2 (LocalVariables|SetOldPitch (Variables|CurrentState|GetPitch)))
        (if (!= (LocalVariables|GetOldPitch) (Math|Float|Clamp(Float) (+ (* (Math|Float|Clamp(Float) (- (Variables|CurrentState|GetTargetPitch) (Variables|CurrentState|GetPitch)) (* _pitchspeedpersec -1.0) _pitchspeedpersec) Delta) _output_get_2) _x _y))
          (bind _output_get_3 (Variables|CurrentState|SetPitch (Math|Float|Clamp(Float) (+ (* (Math|Float|Clamp(Float) (- (Variables|CurrentState|GetTargetPitch) (Variables|CurrentState|GetPitch)) (* _pitchspeedpersec -1.0) _pitchspeedpersec) Delta) _output_get_2) _x _y)))
          (Update|UpdatePitch _output_get_3))))))

(fn GetTargetInfo
  (bind _returnvalue (UserInterface|CreateWidget "/Game/UI/Game/ArrowWidget.ArrowWidget_C"))
  (Default|SetIsEnemy _returnvalue true)
  (bind _output_get (Variables|Default|SetInfoIndicator (Utilities|Struct|MakeTargetInfoStruct _returnvalue (CallFunction|GetShootingSource true))))
  (return _output_get))