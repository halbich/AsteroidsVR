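; Destructible turret that takes hits from BeamActor objects and breaks after a limited number of them.
; Overlaps on the base, torso or guns destroy the beam with an explosion and decrement the remaining hits while the turret is active.
; At zero it scatters explosions around the guns, removes torso and guns, swaps the base to a destroyed material, deactivates and calls TurretDestroyed.
; A separate Hit event only prints a debug string.
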(event OnComponentBeginOverlap(Base)
  (params (OverlappedComponent :type Primitive%20Component%20Object%20Reference) (OtherActor :type Actor%20Object%20Reference) (OtherComp :type Primitive%20Component%20Object%20Reference) (OtherBodyIndex :type Integer) (bFromSweep :type Boolean) (SweepResult :type Hit%20Result%20Structure%20%28by%20ref%29))
  (CallFunction|TryHitwithBeam OtherActor))

(event OnComponentBeginOverlap(Torzo)
  (params (OverlappedComponent :type Primitive%20Component%20Object%20Reference) (OtherActor :type Actor%20Object%20Reference) (OtherComp :type Primitive%20Component%20Object%20Reference) (OtherBodyIndex :type Integer) (bFromSweep :type Boolean) (SweepResult :type Hit%20Result%20Structure%20%28by%20ref%29))
  (CallFunction|TryHitwithBeam OtherActor))

(event OnComponentBeginOverlap(Guns)
  (params (OverlappedComponent :type Primitive%20Component%20Object%20Reference) (OtherActor :type Actor%20Object%20Reference) (OtherComp :type Primitive%20Component%20Object%20Reference) (OtherBodyIndex :type Integer) (bFromSweep :type Boolean) (SweepResult :type Hit%20Result%20Structure%20%28by%20ref%29))
  (CallFunction|TryHitwithBeam OtherActor))

(event EventBeginPlay)

(event EventTick
  (params (DeltaSeconds :type Float%20%28single-precision%29)))

(event Collision|EventHit
  (params (MyComp :type Primitive%20Component%20Object%20Reference) (Other :type Actor%20Object%20Reference) (OtherComp :type Primitive%20Component%20Object%20Reference) (bSelfMoved :type Boolean) (HitLocation :type Vector :default "0, 0, 0") (HitNormal :type Vector :default "0, 0, 0") (NormalImpulse :type Vector :default "0, 0, 0") (Hit :type Hit%20Result%20Structure%20%28by%20ref%29))
  (Development|PrintString "turret hit"))

(fn ConstructionScript)

(fn TryHitwithBeam
  (params (Object :type Object%20Object%20Reference))
  (if (Variables|Default|GetIsActive)
    (bind _asbeam_actor (Utilities|Casting|CastToBeamActor Object))
    (Effects|SpawnEmitteratLocation "/Game/StarterContent/Particles/P_Explosion.P_Explosion" (Transformation|GetActorLocation _asbeam_actor))
    (Actor|DestroyActor _asbeam_actor)
    (bind _result (Math|Integer|DecrementInt (Variables|Default|GetRemainingHits))
      (:%20%20
        (if (<= _result 0)
          (CallFunction|DestroyItself))))))

(fn DestroyItself
  (bind _extendexplosions (Variables|Default|GetExtendExplosions))
  (for _index (range 1 20)
    (Effects|SpawnEmitteratLocation "/Game/StarterContent/Particles/P_Explosion.P_Explosion" (Math|Random|RandomPointinBoundingBox (Transformation|GetWorldLocation (Variables|Default|GetGuns)) (Math|Vector|MakeVector _extendexplosions _extendexplosions _extendexplosions)) (Math|Random|RandomRotator true)))
  (Components|DestroyComponent (Variables|Default|GetTorzo))
  (Rendering|Material|SetMaterial (Variables|Default|GetBase) 0 "/Game/Materials/GameObjects/TurretDestroyed.TurretDestroyed")
  (Variables|Default|SetIsActive false)
  (Default|CallTurretDestroyed))