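; ResultsPawn is the pawn for the game-over results state in an Asteroids game.
; On possession it creates the YouDiedScreen widget and adds it to the player screen.
; Escape, Enter or Space all open the MainMenu level.
; Leftover HUD, game-variant and Kinect error logic remains in the graph but is never executed.
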(event EventPossessed
  (params (NewController :type Controller%20Object%20Reference))
  (bind _returnvalue (UserInterface|CreateWidget "/Game/UMG/Game/YouDiedScreen.YouDiedScreen_C"))
  (UserInterface|Viewport|AddtoPlayerScreen _returnvalue))

(event EventBeginPlay)

(event Input|ActionEvents|InputActionOnEscape
  (params (Key :type Key%20Structure :default "AnyKey"))
  (:Pressed
    (Game|OpenLevel(byName) "MainMenu")))

(event Input|KeyboardEvents|Enter
  (params (Key :type Key%20Structure :default "AnyKey"))
  (:Pressed
    (Game|OpenLevel(byName) "MainMenu")))

(event Input|KeyboardEvents|SpaceBar
  (params (Key :type Key%20Structure :default "AnyKey"))
  (:Pressed
    (Game|OpenLevel(byName) "MainMenu")))

(fn ConstructionScript)