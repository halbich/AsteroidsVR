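; Gate is a ring-shaped target that deactivates when a FlyingPawn overlaps it.
; The construction script spaces instanced meshes evenly around a circle from Points and Scale, and sizes the Cylinder to match.
; GetTargetInfo creates a non-enemy arrow widget and pairs it with the gate's location as its indicator info.
; On overlap, the gate switches to its inactive material and passes that info through GotInactive.
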(event EventBeginPlay)

(event Collision|EventActorBeginOverlap
  (params (OtherActor :type Actor%20Object%20Reference))
  (Utilities|Casting|CastToFlyingPawn OtherActor)
  (Variables|Default|SetIsActive false)
  (Rendering|Material|SetMaterial (Variables|Default|GetInstancedStaticMesh) 0 "/Game/Materials/GameObjects/GateInactive.GateInactive")
  (Default|CallGotInactive (Variables|Default|GetInfoIndicator)))

(event EventTick
  (params (DeltaSeconds :type Float%20%28single-precision%29)))

(fn ConstructionScript
  (bind _scale (Variables|Default|GetScale))
  (bind _points (Variables|Default|GetPoints))
  (bind _returnvalue (+ _scale 1e+01))
  (bind _returnvalue_2 (* _returnvalue 0.02))
  (LocalVariables|SetRotStep (/ 1.0 (Math|Conversions|ToFloat(Integer) _points)))
  (for _index (range 0 (- _points 1))
    (Components|InstancedStaticMesh|AddInstance (Variables|Default|GetInstancedStaticMesh) (Math|Transform|MakeTransform (Math|Vector|RotateVector (Math|Vector|MakeVector 0.0 (Variables|Default|GetScale) 0.0) (Math|Rotator|MakeRotator (* (* _index (LocalVariables|GetRotStep)) 3.6e+02) 0.0 0.0))))
    (Transformation|SetRelativeScale3D (Variables|Default|GetCylinder) (Math|Vector|MakeVector _returnvalue_2 _returnvalue_2 1.0))))

(fn GetTargetInfo
  (bind _returnvalue (UserInterface|CreateWidget "/Game/UMG/Game/ArrowWidget.ArrowWidget_C"))
  (Default|SetIsEnemy _returnvalue false)
  (bind _output_get (Variables|Default|SetInfoIndicator (Utilities|Struct|MakeTargetInfoStruct _returnvalue (Transformation|GetWorldLocation (Variables|Default|GetDefaultSceneRoot self)))))
  (return _output_get))