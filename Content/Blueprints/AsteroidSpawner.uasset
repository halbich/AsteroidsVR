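; Asteroid spawner actor that scatters a random number of asteroid meshes around its location to form a field.
; The construction script adds each as an InstancedStaticMesh instance in world space, with random position, rotation and uniform scale, so the layout re-randomizes whenever construction reruns.
; Despite its name, SphereSize sets the half-extent of a cubic volume.
; The event graph holds no active logic.
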(event EventBeginPlay)

(event Collision|EventActorBeginOverlap
  (params (OtherActor :type Actor%20Object%20Reference)))

(event EventTick
  (params (DeltaSeconds :type Float%20%28single-precision%29)))

(fn ConstructionScript
  (bind _spheresize (LocalVariables|GetsphereSize))
  (for _index (range 1 (Math|Random|RandomIntegerinRange (Variables|Default|GetMinAsterids) (Variables|Default|GetMaxAsterids)))
    (bind _output_get (LocalVariables|SetcurrentRandomSize (Math|Random|RandomFloatinRange 4e+01 1.5e+02)))
    (Class|InstancedStaticMeshComponent|AddInstanceWorldSpace (Variables|Default|GetInstancedStaticMesh) (Math|Transform|MakeTransform (Math|Random|RandomPointinBoundingBox (Transformation|GetActorLocation) (Math|Vector|MakeVector _spheresize _spheresize _spheresize)) (Math|Random|RandomRotator true) (Math|Vector|MakeVector _output_get _output_get _output_get)))))