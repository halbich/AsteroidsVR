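; Kinect controller that drives pose calibration and live body-pose input for an Asteroids game, active only in one game variant.
; Each tick it reports sensor and tracking changes, then samples pitch-adjusted joints of the centered body into a measure.
; Game measures update KinectSetup's live pose; calibration measures feed visualizers and accumulate.
; Each config section's end passes the most centered sample to KinectSetup as that pose, and FinalizeConfig completes setup.
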(event EventBeginPlay
  (bind _asasterorids_game_instance (Utilities|Casting|CastToAsteroridsGameInstance (Game|GetGameInstance)))
  (Variables|Default|SetUpdateKinectData (Utilities|Enum|Equal(Enum) (Variables|/Game/Blueprints/AsteroridsGameInstance.AsteroridsGameInstance_C|GetGameVariant _asasterorids_game_instance) "NewEnumerator1"))
  (bind _outactors (Actor|GetAllActorsOfClass "/Game/Blueprints/Kinect/KinectVisualizer.KinectVisualizer_C"))
  (bind _output_get (Variables|Default|SetVizualizers _outactors))
  (Development|PrintString (Utilities|String|ToString(Integer) (Utilities|Array|Length _output_get))))

(event EventTick
  (params (DeltaSeconds :type Float%20%28single-precision%29))
  (if (Variables|Default|GetUpdateKinectData)
    (CallFunction|CheckKinect)
    (CallFunction|SetWatchedBody)
    (if (Math|Boolean|ANDBoolean (Variables|Default|GetIsKinectAwake) (Variables|Default|GetBodyTracked) (Utilities|Enum|NotEqual(Enum) (Variables|Default|GetCurrentMeasuredData) "Null"))
      (CallFunction|DoMeasure))))

(fn ConstructionScript)

(fn ConfigSectionBegin
  (params (Section :type Kinect%20Setup%20Config%20Section%20Structure))
  (Variables|Default|SetCurrentMeasuredData (.MeasureType (Utilities|Struct|BreakKinectSetupConfigSection Section))))

(fn ConfigSectionEnd
  (bind _measures (Variables|Default|GetMeasures))
  (if (Utilities|Enum|NotEqual(Enum) (Variables|Default|GetCurrentMeasuredData) "Null")
    (bind _returnvalue (Class|MyBPFunctionLibrary|GetMostCenteredPosition _measures))
    (Class|KinectSetupComponent|NotePose (Variables|Default|GetKinectSetup) _returnvalue (Variables|Default|GetCurrentMeasuredData))
    (Utilities|Array|Clear _measures)))

(fn DoMeasure
  (LocalVariables|SetCurrent (Class|MyBPFunctionLibrary|GetEmptyMeasure))
  (for _array_element (Variables|Default|GetWatchingJoints)
    (bind _returnvalue (Class|KinectInterfaceComponent|GetPitchAdjustedJointPosition (Variables|Default|GetKinectInterface) _array_element (Variables|Default|GetCenteredBody)))
    (Class|MyBPFunctionLibrary|UpdateValue (LocalVariables|GetCurrent) _returnvalue (Utilities|MapEnums _array_element)))
  (if (Utilities|Enum|Equal(Enum) (Variables|Default|GetCurrentMeasuredData) "Game")
    (Class|KinectSetupComponent|UpdateGamePose (Variables|Default|GetKinectSetup) (LocalVariables|GetCurrent))
    (else
      (Utilities|Array|Add (Variables|Default|GetMeasures) (LocalVariables|GetCurrent))
      (CallFunction|UpdateVizualizer (LocalVariables|GetCurrent)))))

(fn SetWatchedBody
  (bind (_centeredbody _istracked) (Class|KinectInterfaceComponent|GetCenteredBody (Variables|Default|GetKinectInterface)))
  (if _istracked
    (Variables|Default|SetCenteredBody _centeredbody))
  (if (Math|Boolean|NotEqual(Boolean) _istracked (Variables|Default|GetBodyTracked))
    (bind _output_get (Variables|Default|SetBodyTracked _istracked))
    (Default|CallBodyTrackedChanged _output_get)))

(fn CheckKinect
  (bind _returnvalue (Class|KinectInterfaceComponent|IsKinectAwake (Variables|Default|GetKinectInterface)))
  (if (Math|Boolean|NotEqual(Boolean) _returnvalue (Variables|Default|GetIsKinectAwake))
    (bind _output_get (Variables|Default|SetIsKinectAwake _returnvalue))
    (Default|CallKinectAwakeChanged _output_get)
    (if _output_get
      (Default|CallBodyTrackedChanged false))))

(fn UpdateVizualizer
  (params (Measure :type Custom%20Kinect%20Measure%20Structure))
  (for _array_element (Variables|Default|GetVizualizers)
    (Default|UpdateSpheres _array_element Measure)))

(fn FinalizeConfig
  (Class|KinectSetupComponent|FinalizeConfiguration (Variables|Default|GetKinectSetup)))