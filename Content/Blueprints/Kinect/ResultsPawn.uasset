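; ResultsPawn is a pawn in a Kinect-enabled asteroids game that presents the post-death results screen.
; On possession it creates a YouDiedScreen widget and adds it to the player screen, and Escape returns to the MainMenu level.
; Leftover, never-executed nodes handle HUD setup, game-variant section start and Kinect tracking error messages.
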(event EventPossessed
  (params (NewController :type Controller%20Object%20Reference))
  (bind _returnvalue (UserInterface|CreateWidget "/Game/UI/Game/YouDiedScreen.YouDiedScreen_C"))
  (UserInterface|Viewport|AddtoPlayerScreen _returnvalue))

(event EventBeginPlay)

(event Input|KeyboardEvents|Escape
  (params (Key :type Key%20Structure :default "AnyKey"))
  (:Pressed
    (Game|OpenLevel(byName) "MainMenu")))

(fn ConstructionScript)