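; Pawn that runs the Kinect calibration sequence in a config widget before gameplay, with Escape returning to the main menu.
; On possession it creates the HUD and, depending on the game variant, either runs all config sections or skips to the last.
; Tick advances each timed section while Kinect is ready, updating the progress bar and notifying the KinectController at section boundaries.
; Lost body tracking or sensor connection shows errors; completion finalizes config and fires a measure-end event.
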(event Custom|OnBodyTrackedChanged
  (params (BodyTracked :type Boolean))
  (if (Variables|Default|GetIsMeasureInProgress)
    (Default|SetError (Variables|Default|GetHUD) "Tracked body is no longer aviable" BodyTracked)
    (Variables|Default|SetKinectReady BodyTracked)))

(event Custom|OnKinectAwakeChanged
  (params (KinectAwake :type Boolean))
  (Default|SetError (Variables|Default|GetHUD) "Kinect is not connected! 
Please reconnect your device." KinectAwake)
  (Variables|Default|SetKinectReady KinectAwake))

(event EventPossessed
  (params (NewController :type Controller%20Object%20Reference))
  (bind _askinect_controller (Utilities|Casting|CastToKinectController NewController))
  (Variables|Default|SetKinectController _askinect_controller)
  (bind _returnvalue (UserInterface|CreateWidget "/Game/UMG/Game/ConfigWidget.ConfigWidget_C"))
  (bind _output_get (Variables|Default|SetHUD _returnvalue))
  (UserInterface|Viewport|AddtoPlayerScreen _output_get)
  (bind _asasterorids_game_instance (Utilities|Casting|CastToAsteroridsGameInstance (Game|GetGameInstance)))
  (if (Utilities|Enum|Equal(Enum) (Variables|/Game/Blueprints/Common/AsteroridsGameInstance.AsteroridsGameInstance_C|GetGameVariant _asasterorids_game_instance) "NewEnumerator1")
    _
    (else
      (Variables|Sections|SetCurrentSectionID (- (Utilities|Array|Length (Variables|Sections|GetConfigSections)) 1))))
  (CallFunction|StartSection))

(event EventBeginPlay
  (bind _kinectcontroller (Variables|Default|GetKinectController))
  (if (and (Utilities|IsValid _kinectcontroller) (Variables|/Game/Blueprints/Kinect/KinectController.KinectController_C|GetUpdateKinectData _kinectcontroller))
    (EventDispatchers|BindEventtoBodyTrackedChanged _kinectcontroller (delegate Custom|OnBodyTrackedChanged))
    (EventDispatchers|BindEventtoKinectAwakeChanged _kinectcontroller (delegate Custom|OnKinectAwakeChanged))))

(event EventTick
  (params (DeltaSeconds :type Float%20%28single-precision%29))
  (Utilities|IsValid (Variables|Default|GetHUD)
    (:Is%20Valid
      (Utilities|IsValid (Variables|Default|GetKinectController)
        (:Is%20Valid
          (CallFunction|UpdateConfig DeltaSeconds))))))

(event EventUnpossessed
  (params (OldController :type Controller%20Object%20Reference))
  (bind _hud (Variables|Default|GetHUD))
  (Utilities|IsValid _hud
    (:Is%20Valid
      (Widget|RemovefromParent _hud))))

(event Input|KeyboardEvents|Escape
  (params (Key :type Key%20Structure :default "AnyKey"))
  (:Pressed
    (Game|OpenLevel(byName) "MainMenu")))

(fn ConstructionScript
  (Variables|Sections|SetConfigSections (Class|MyBPFunctionLibrary|GetDefaultKinectConfigSetup)))

(fn UpdateConfig
  (params (Delta :type Float%20%28single-precision%29))
  (bind _currentsectionduration (Variables|Sections|GetCurrentSectionDuration))
  (if (and (Variables|Default|GetIsMeasureInProgress) (or (not (Variables|/Game/Blueprints/Kinect/KinectController.KinectController_C|GetUpdateKinectData (Variables|Default|GetKinectController))) (Variables|Default|GetKinectReady)))
    (bind _output_get (Variables|Sections|SetCurrentSectionProgress (+ Delta (Variables|Sections|GetCurrentSectionProgress))))
    (if (> _currentsectionduration 0.0)
      (if (>= _output_get _currentsectionduration)
        (CallFunction|FinishSection)
        (else
          (Misc|InitConfigUpdateProgressBar))))))

(fn StartSection
  (bind _configsections (Variables|Sections|GetConfigSections))
  (bind _returnvalue (Utilities|Array|Length _configsections))
  (if (< (Variables|Sections|GetCurrentSectionID) _returnvalue)
    (SectionInit|InitConfig)
    (if (== (Variables|Sections|GetCurrentSectionID) (- _returnvalue 1))
      (Default|StartFadein (Variables|Default|GetHUD)))
    (else
      (SectionPlayGame|StartPlaying))))

(fn StartPlaying
  (bind _kinectcontroller (Variables|Default|GetKinectController))
  (Utilities|IsValid _kinectcontroller
    (:Is%20Valid
      (Default|FinalizeConfig _kinectcontroller))
    (:Is%20Not%20Valid
      _))
  (Default|CallOnMeasureEnd))

(fn FinishSection
  (Default|ConfigSectionEnd (Variables|Default|GetKinectController))
  (Variables|Default|SetIsMeasureInProgress false)
  (Math|Integer|IncrementInt (Variables|Sections|GetCurrentSectionID)
    (:%20%20
      (CallFunction|StartSection))))

(fn Clear
  (bind _hud (Variables|Default|GetHUD))
  (Utilities|IsValid _hud
    (:Is%20Valid
      (Default|Clear _hud)
      (bind _output_get (Variables|Sections|SetCurrentSectionProgress 0.0))
      (bind _output_get_2 (Variables|Sections|SetCurrentSectionDuration _output_get))
      (Misc|SafeSetMessage)
      (Misc|SafeSetPercentil _output_get_2))))

(fn SafeSetMessage
  (params (Text :type Text))
  (bind _hud (Variables|Default|GetHUD))
  (Utilities|IsValid _hud
    (:Is%20Valid
      (Variables|/Game/UMG/Game/ConfigWidget.ConfigWidget_C|SetText _hud Text))))

(fn InitConfigUpdateProgressBar
  (Misc|SafeSetPercentil (/ (Variables|Sections|GetCurrentSectionProgress) (Variables|Sections|GetCurrentSectionDuration))))

(fn SafeSetPercentil
  (params (Percentil :type Float%20%28single-precision%29))
  (bind _hud (Variables|Default|GetHUD))
  (Utilities|IsValid _hud
    (:Is%20Valid
      (Progress|SetPercent (Variables|/Game/UMG/Game/ConfigWidget.ConfigWidget_C|GetMainProgressBar _hud) Percentil))))

(fn SafeShowProgressBar
  (bind _hud (Variables|Default|GetHUD))
  (Utilities|IsValid _hud
    (:Is%20Valid
      (Default|ShowProgressBar _hud))))

(fn InitConfig
  (bind _currentsectionid (Variables|Sections|GetCurrentSectionID))
  (bind _configsections (Variables|Sections|GetConfigSections))
  (bind _item (Utilities|Array|Get(acopy) _configsections _currentsectionid))
  (bind (_measuretext _measureduration _showprogressbar) (Utilities|Struct|BreakKinectSetupConfigSection _item))
  (Misc|Clear)
  (Variables|Sections|SetCurrentSectionDuration _measureduration)
  (Misc|SafeSetMessage _measuretext)
  (if _showprogressbar
    (Misc|SafeShowProgressBar))
  (Variables|Default|SetIsMeasureInProgress true)
  (Default|ConfigSectionBegin (Variables|Default|GetKinectController) _item))