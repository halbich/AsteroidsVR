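; KinectVisualizer displays a Kinect body measurement as a set of static mesh markers, one per upper-body joint.
; UpdateSpheres receives a measure and loops over twelve joints covering spine, neck, head, and both arms down to the hands.
; Paired Select nodes match each mesh component to its joint position, which becomes that component's relative location without sweeping.
; The construction script is empty.
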(fn ConstructionScript)

(fn UpdateSpheres
  (params (Measure :type Custom%20Kinect%20Measure%20Structure))
  (bind (_baseofspine _middlefspine _neck _head _leftshoulder _leftelbow _leftwrist _lefthand _rightshoulder _rightelbow _rightwrist _righthand) (Utilities|Struct|BreakCustomKinectMeasure Measure))
  (for _index (range 0 11)
    (Transformation|SetRelativeLocation (Utilities|Select :Index _index :Option%200 (Variables|Default|GetStaticMesh) :Option%201 (Variables|Default|GetStaticMesh1) :Option%202 (Variables|Default|GetStaticMesh2) :Option%203 (Variables|Default|GetStaticMesh3) :Option%204 (Variables|Default|GetStaticMesh4) :Option%205 (Variables|Default|GetStaticMesh5) :Option%206 (Variables|Default|GetStaticMesh6) :Option%207 (Variables|Default|GetStaticMesh7) :Option%208 (Variables|Default|GetStaticMesh8) :Option%209 (Variables|Default|GetStaticMesh9) :Option%2010 (Variables|Default|GetStaticMesh10) :Option%2011 (Variables|Default|GetSphere)) (Utilities|Select :Index _index :Option%200 _baseofspine :Option%201 _middlefspine :Option%202 _neck :Option%203 _head :Option%204 _leftshoulder :Option%205 _leftelbow :Option%206 _leftwrist :Option%207 _lefthand :Option%208 _rightshoulder :Option%209 _rightelbow :Option%2010 _rightwrist :Option%2011 _righthand) false false)))