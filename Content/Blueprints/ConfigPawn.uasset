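; Pawn that runs a timed Kinect configuration sequence before play, showing each section's message and progress on a ConfigWidget.
; On possession it caches the KinectController and starts the ConfigSections sequence, jumping to the last section unless the game variant matches one specific value.
; Tick advances the timer and tracked-body count, while section begin and end are reported to the controller.
; The last section fades in the HUD, then OnMeasureEnd is called.
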(event EventBeginPlay)

(event Collision|EventActorBeginOverlap
  (params (OtherActor :type Actor%20Object%20Reference)))

(event EventPossessed
  (params (NewController :type Controller%20Object%20Reference))
  (Development|PrintString "Config possesed")
  (bind _askinect_controller (Utilities|Casting|CastToKinectController NewController))
  (Variables|Default|SetKinectController _askinect_controller)
  (bind _returnvalue (UserInterface|CreateWidget "/Game/UI/Game/ConfigWidget.ConfigWidget_C"))
  (bind _output_get (Variables|Default|SetHUD _returnvalue))
  (UserInterface|Viewport|AddtoPlayerScreen _output_get)
  (bind _asasterorids_game_instance (Utilities|Casting|CastToAsteroridsGameInstance (Game|GetGameInstance)))
  (if (Utilities|Enum|Equal(Enum) (Variables|/Game/Blueprints/AsteroridsGameInstance.AsteroridsGameInstance_C|GetGameVariant _asasterorids_game_instance) "NewEnumerator1")
    _
    (else
      (Variables|Sections|SetCurrentSectionID (- (Utilities|Array|Length (Variables|Sections|GetConfigSections)) 1))))
  (CallFunction|StartSection))

(event EventTick
  (params (DeltaSeconds :type Float%20%28single-precision%29))
  (bind _kinectcontroller (Variables|Default|GetKinectController))
  (Utilities|IsValid (Variables|Default|GetHUD)
    (:Is%20Valid
      (Utilities|IsValid _kinectcontroller
        (:Is%20Valid
          (CallFunction|UpdateConfig DeltaSeconds)
          (bind _returnvalue (Class|KinectInterfaceComponent|GetTrackedBodies (Variables|/Game/Blueprints/Kinect/KinectController.KinectController_C|GetKinectInterface _kinectcontroller)))
          (Variables|/Game/UI/Game/ConfigWidget.ConfigWidget_C|SetBodiesCount (Variables|Default|GetHUD) (Utilities|Array|Length _returnvalue)))))))

(event EventUnpossessed
  (params (OldController :type Controller%20Object%20Reference))
  (bind _hud (Variables|Default|GetHUD))
  (Development|PrintString "config unpossesed")
  (Utilities|IsValid _hud
    (:Is%20Valid
      (Widget|RemovefromParent _hud))))

(fn ConstructionScript)

(fn UpdateConfig
  (params (Delta :type Float%20%28single-precision%29))
  (bind _currentsectionduration (Variables|Sections|GetCurrentSectionDuration))
  (if (Variables|Default|GetIsMeasureInProgress)
    (bind _output_get (Variables|Sections|SetCurrentSectionProgress (+ Delta (Variables|Sections|GetCurrentSectionProgress))))
    (if (> _currentsectionduration 0.0)
      (if (>= _output_get _currentsectionduration)
        (CallFunction|FinishSection)
        (else
          (Misc|InitConfigUpdateProgressBar)))
      (else
        (Development|PrintString "dur 0" true true "(R=0.000000,G=0.660000,B=1.000000,A=1.000000)" 0.1)))))

(fn StartSection
  (bind _configsections (Variables|Sections|GetConfigSections))
  (bind _returnvalue (Utilities|Array|Length _configsections))
  (if (< (Variables|Sections|GetCurrentSectionID) _returnvalue)
    (SectionInit|InitConfig)
    (if (== (Variables|Sections|GetCurrentSectionID) (- _returnvalue 1))
      (Default|StartFadein (Variables|Default|GetHUD)))
    (else
      (SectionPlayGame|StartPlaying))))

(fn StartPlaying
  (Default|CallOnMeasureEnd)
  (Development|PrintString "Hello, start"))

(fn FinishSection
  (Default|ConfigSectionEnd (Variables|Default|GetKinectController))
  (Variables|Default|SetIsMeasureInProgress false)
  (Math|Integer|IncrementInt (Variables|Sections|GetCurrentSectionID)
    (:%20%20
      (CallFunction|StartSection))))

(fn Clear
  (bind _hud (Variables|Default|GetHUD))
  (Utilities|IsValid _hud
    (:Is%20Valid
      (Default|Clear _hud)
      (bind _output_get (Variables|Sections|SetCurrentSectionProgress 0.0))
      (bind _output_get_2 (Variables|Sections|SetCurrentSectionDuration _output_get))
      (Misc|SafeSetMessage)
      (Misc|SafeSetPercentil _output_get_2))))

(fn SafeSetMessage
  (params (Text :type Text))
  (bind _hud (Variables|Default|GetHUD))
  (Utilities|IsValid _hud
    (:Is%20Valid
      (Variables|/Game/UI/Game/ConfigWidget.ConfigWidget_C|SetText _hud Text))))

(fn InitConfigUpdateProgressBar
  (Misc|SafeSetPercentil (/ (Variables|Sections|GetCurrentSectionProgress) (Variables|Sections|GetCurrentSectionDuration))))

(fn SafeSetPercentil
  (params (Percentil :type Float%20%28single-precision%29))
  (bind _hud (Variables|Default|GetHUD))
  (Utilities|IsValid _hud
    (:Is%20Valid
      (Progress|SetPercent (Variables|/Game/UI/Game/ConfigWidget.ConfigWidget_C|GetMainProgressBar _hud) Percentil))))

(fn SafeShowProgressBar
  (bind _hud (Variables|Default|GetHUD))
  (Utilities|IsValid _hud
    (:Is%20Valid
      (Default|ShowProgressBar _hud))))

(fn InitConfig
  (bind _currentsectionid (Variables|Sections|GetCurrentSectionID))
  (bind _configsections (Variables|Sections|GetConfigSections))
  (bind _item (Utilities|Array|Get(acopy) _configsections _currentsectionid))
  (bind (_measuretext _measureduration _showprogressbar) (Utilities|Struct|BreakConfigSection _item))
  (Misc|Clear)
  (Variables|Sections|SetCurrentSectionDuration _measureduration)
  (Misc|SafeSetMessage _measuretext)
  (if _showprogressbar
    (Misc|SafeShowProgressBar))
  (Variables|Default|SetIsMeasureInProgress true)
  (Default|ConfigSectionBegin (Variables|Default|GetKinectController) _item))